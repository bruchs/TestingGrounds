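; NPC AI controller that runs patrol behavior for its controlled pawn.
; On BeginPlay it sets up the Patrol_BB blackboard and runs the Patrol_BT behavior tree.
; Its AI Perception update handler only prints the pawn, sense class and perceived actor as debug text, without writing to the blackboard.
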(event `self.ReceiveBeginPlay`
  (`self.UseBlackboard` "/Game/Blueprints/AI/Patrol_BB.Patrol_BB")
  (`self.RunBehaviorTree` "/Game/Blueprints/AI/Patrol_BT.Patrol_BT"))

(event `self.AIPerception.OnTargetPerceptionUpdated`
  (params (Actor :type "Actor Object Reference") (Stimulus :type "AIStimulus Structure"))
  (bind _returnvalue (`AIPerceptionSystem.GetSenseClassForStimulus` Stimulus))
  (`KismetSystemLibrary.PrintString` (`KismetStringLibrary.Concat_StrStr` (`KismetSystemLibrary.GetDisplayName` (`self.K2_GetPawn` self)) " " (`KismetSystemLibrary.GetClassDisplayName` _returnvalue) " " (`KismetSystemLibrary.GetDisplayName` Actor))))

(fn `UserConstructionScript`)